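; Collectible treasure pickup that adds a random amount of treasure points to the player on touch.
; On BeginPlay it rolls its value between configurable minimum and maximum bounds.
; Overlap by an actor tagged Player adds that value to TreasurePoints on the player's BP_ThirdPersonCharacter, then destroys the pickup.
; Tick spins the placeholder cube by a fixed step each frame, independent of delta time.
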(event EventBeginPlay
  (Variables|Default|Setthis_treasure (Math|Random|RandomIntegerinRange (Variables|Default|Getmin_treasure) (Variables|Default|Getmax_treasure))))

(event Collision|EventActorBeginOverlap
  (params (OtherActor :type Actor%20Object%20Reference))
  (if (Actor|ActorHasTag OtherActor "Player")
    (bind _asbp_third_person_character (Utilities|Casting|CastToBP_ThirdPersonCharacter (Game|GetPlayerCharacter 0)))
    (Variables|/Game/Test/ThirdPerson/Blueprints/BP_ThirdPersonCharacter.BP_ThirdPersonCharacter_C|Settreasure_points _asbp_third_person_character (+ (Variables|/Game/Test/ThirdPerson/Blueprints/BP_ThirdPersonCharacter.BP_ThirdPersonCharacter_C|Gettreasure_points _asbp_third_person_character) (Variables|Default|Getthis_treasure)))
    (Actor|DestroyActor)))

(event EventTick
  (params (DeltaSeconds :type Float%20%28single-precision%29))
  (Transformation|AddLocalRotation (Variables|Default|GetPlaceholder_Cube) "0.000000,0.200000,0.000000" false false))

(fn ConstructionScript)