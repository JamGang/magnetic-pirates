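; BP_Maelstroms is an unfinished maelstrom hazard that reacts when the player's ship overlaps its sphere collision.
; On overlap it saves the player's transform, then calls AttackShip while the distance to its center exceeds zero.
; AttackShip applies a capsule force along the center-to-player direction, currently multiplied by zero, and zeroes the player's rotation.
; The point penalty, relocation and end-overlap cleanup are only debug-print placeholders or unset calls.
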(event OnComponentBeginOverlap(SphereCollision)
  (params (OverlappedComponent :type Primitive%20Component%20Object%20Reference) (OtherActor :type Actor%20Object%20Reference) (OtherComp :type Primitive%20Component%20Object%20Reference) (OtherBodyIndex :type Integer) (bFromSweep :type Boolean) (SweepResult :type Hit%20Result%20Structure%20%28by%20ref%29))
  (bind _returnvalue (Game|GetPlayerCharacter 0))
  ;[0.15 0.15 0.15 0.5] On overlap with ship
  (if (== OtherActor _returnvalue)
    (Utilities|FlowControl|Sequence
      (:then_0
        (Variables|Default|SetPlayerInitialTransform (Transformation|GetActorTransform _returnvalue)))
      (:then_1
        (if (> (Math|Vector|Distance(Vector) (Transformation|GetActorLocation _returnvalue) (Transformation|GetActorLocation)) 0.0)
          (CallFunction|AttackShip)
          (else
            (Development|PrintString "Remove 1 point and move ship to the opposite end of initial transform")
            (Transformation|SetActorLocationAndRotation (Game|GetPlayerCharacter 0) "0, 0, 0")))))
    (else
      (Development|PrintString "Wrong Component"))))

(event OnComponentEndOverlap(SphereCollision)
  (params (OverlappedComponent :type Primitive%20Component%20Object%20Reference) (OtherActor :type Actor%20Object%20Reference) (OtherComp :type Primitive%20Component%20Object%20Reference) (OtherBodyIndex :type Integer))
  (Development|PrintString "Stop spinning? Delte from world?"))

(event Custom|AttackShip
  (bind _returnvalue (Game|GetPlayerCharacter 0))
  ;[0.15 0.15 0.15 0.5] On overlap with ship
  ;;[0.15 0.15 0.15 0.5] Attack Ship
  (Physics|AddForce (Variables|/Script/Engine.Character|GetCapsuleComponent _returnvalue) (* (Math|Vector|Normalize (- (Transformation|GetActorLocation (Game|GetPlayerCharacter 0)) (Transformation|GetActorLocation))) "") "None" false)
  (Transformation|SetActorRotation _returnvalue))

(fn ConstructionScript)