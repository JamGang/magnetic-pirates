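; BP_PlayerCharacter is the player character, handling basic movement through Enhanced Input.
; On BeginPlay it casts its controller to BP_PlayerController and adds the input mapping context.
; Forward and right input actions feed AddMovementInput along the capsule's forward and right vectors, both scaled by the action value's Y component.
; Each movement event also prints the actor's X and Y location as debug output.
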(event Input|EnhancedActionEvents|EnhancedInputActionIA_PlayerMovement_Forward
  (params (ActionValue :type Vector%202D%20Structure) (ElapsedSeconds :type Float%20%28double-precision%29) (TriggeredSeconds :type Float%20%28double-precision%29) (InputAction :type Input%20Action%20Object%20Reference :default "/Game/Input/IA_PlayerMovement_Forward.IA_PlayerMovement_Forward"))
  (bind _returnvalue (Transformation|GetActorLocation))
  ;[0.15 0.15 0.15 0.5] PlayerInput
  (Pawn|Input|AddMovementInput (Math|Vector|GetForwardVector (Variables|Collision|GetCapsuleComponent)) (.Y (Math|Vector2D|BreakVector2D ActionValue)) false)
  (Development|PrintString (Utilities|String|ToString(Float) (.x _returnvalue)))
  (Development|PrintString (Utilities|String|ToString(Float) (.y _returnvalue)) true true "(R=0.000000,G=0.660000,B=1.000000,A=1.000000)" (.y _returnvalue)))

(event Input|EnhancedActionEvents|EnhancedInputActionIA_PlayerMovement_Right
  (params (ActionValue :type Vector%202D%20Structure) (ElapsedSeconds :type Float%20%28double-precision%29) (TriggeredSeconds :type Float%20%28double-precision%29) (InputAction :type Input%20Action%20Object%20Reference :default "/Game/Input/IA_PlayerMovement_Right.IA_PlayerMovement_Right"))
  (bind _returnvalue (Transformation|GetActorLocation))
  ;[0.15 0.15 0.15 0.5] PlayerInput
  (Pawn|Input|AddMovementInput (Math|Vector|GetRightVector (Variables|Collision|GetCapsuleComponent)) (.Y (Math|Vector2D|BreakVector2D ActionValue)) false)
  (Development|PrintString (Utilities|String|ToString(Float) (.x _returnvalue)))
  (Development|PrintString (Utilities|String|ToString(Float) (.y _returnvalue))))

(event EventBeginPlay
  ;[0.15 0.15 0.15 0.5] OnBegin
  (bind _asbp_player_controller (Utilities|Casting|CastToBP_PlayerController (Pawn|GetController)))
  (Utilities|IsValid (PlayerController|LocalPlayerSubsystems|GetEnhancedInputLocalPlayerSubsystem _asbp_player_controller)
    (:Is%20Valid
      (Input|AddMappingContext (PlayerController|LocalPlayerSubsystems|GetEnhancedInputLocalPlayerSubsystem _asbp_player_controller) "/Game/Input/InputMapping.InputMapping" 0 "(bIgnoreAllPressedKeysUntilRelease=True,bForceImmediately=False,bNotifyUserSettings=False)"))))

(fn ConstructionScript)